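; BP_Gates is a double gate that opens once for a main character carrying both sword and shield, and closes behind them.
; Overlap triggers call Open and Close, each guarded by a DoOnce, to play or reverse a timeline that lerps both gate roots' yaw.
; BeginPlay captures the closed yaws and derives the play rate from TimeToOpen.
; The close trigger also deactivates the character's Rain component.
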(event `self.ReceiveBeginPlay`
  (bind (_returnvalue_roll _returnvalue_pitch _returnvalue_yaw) (`KismetMathLibrary.BreakRotator` (`SceneComponent.K2_GetComponentRotation` (`self.GateRoot`))))
  (bind (_returnvalue_roll_2 _returnvalue_pitch_2 _returnvalue_yaw_2) (`KismetMathLibrary.BreakRotator` (`SceneComponent.K2_GetComponentRotation` (`self.GateRoot1`))))
  (`TimelineComponent.SetPlayRate` (`self.Gate_RL`) (/ 1.0 (`self.Time to open`)))
  (set `self.ClosePosition_first` _returnvalue_yaw)
  (set `self.ClosePosition_secont` _returnvalue_yaw_2))

(event `Open`
  (`/Engine/EditorBlueprintResources/StandardMacros.DoOnce` false
    (:`Completed`
      (bind (_direction _door_track) (`Timeline|Gate_RL` :!via `PlayFromStart` :!label _label)
        (:`Update`
          (`SceneComponent.K2_SetWorldRotation` (`self.GateRoot`) (`KismetMathLibrary.MakeRotator` 0.0 0.0 (`KismetMathLibrary.Lerp` (`self.ClosePosition_first`) (`self.OpenPosition_first`) _door_track)) false false)
          (`SceneComponent.K2_SetWorldRotation` (`self.GateRoot1`) (`KismetMathLibrary.MakeRotator` 0.0 0.0 (`KismetMathLibrary.Lerp` (`self.ClosePosition_secont`) (`self.OpenPosition_second`) _door_track)) false false))))))

(event `Close`
  (`/Engine/EditorBlueprintResources/StandardMacros.DoOnce` false
    (:`Completed`
      (goto _label :!via `Reverse`))))

(event `self.OpenTrigger.OnComponentBeginOverlap`
  (params (OverlappedComponent :type "PrimitiveComponent Object Reference") (OtherActor :type "Actor Object Reference") (OtherComp :type "PrimitiveComponent Object Reference") (OtherBodyIndex :type Integer) (bFromSweep :type Boolean) (SweepResult :type "HitResult Structure (by ref)"))
  (bind _asmain_character (cast `/Game/Main/Character/MainCharacter` OtherActor))
  (if (`KismetSystemLibrary.IsValid` _asmain_character)
    (if (`/Game/Main/Character/MainCharacter.HaveSword?` _asmain_character)
      (if (`/Game/Main/Character/MainCharacter.HaveShield?` _asmain_character)
        (`self.Open`)))))

(event `self.CloseTriger.OnComponentBeginOverlap`
  (params (OverlappedComponent :type "PrimitiveComponent Object Reference") (OtherActor :type "Actor Object Reference") (OtherComp :type "PrimitiveComponent Object Reference") (OtherBodyIndex :type Integer) (bFromSweep :type Boolean) (SweepResult :type "HitResult Structure (by ref)"))
  (bind _asmain_character (cast `/Game/Main/Character/MainCharacter` OtherActor))
  (if (`KismetSystemLibrary.IsValid` _asmain_character)
    (`self.Close`)
    (`ActorComponent.Deactivate` (`/Game/Main/Character/MainCharacter.Rain` _asmain_character))))

(fn `UserConstructionScript`)