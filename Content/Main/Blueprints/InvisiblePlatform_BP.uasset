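; InvisiblePlatform_BP is a platform actor whose particle effects blink on and off continuously during play.
; On BeginPlay it gathers its particle system components into the Effects array, then starts the Blinking event.
; Blinking deactivates the effects, reactivates them after a delay, then calls itself after another delay.
; The Delays sit inside the deactivation loop body, so the cycle relies on Delay ignoring repeat triggers while pending.
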(event `Write Array`
  (set `self.Effects` (`|MakeArray` (`self.ParticleSystem`) (`self.ParticleSystem1`) (`self.ParticleSystem2`) (`self.ParticleSystem3`) (`self.ParticleSystem4`) (`self.ParticleSystem5`) (`self.ParticleSystem6`) (`self.ParticleSystem7`) (`self.ParticleSystem8`) (`self.ParticleSystem9`) (`self.ParticleSystem10`) (`self.ParticleSystem11`) (`self.ParticleSystem12`) (`self.ParticleSystem13`) (`self.ParticleSystem14`) (`self.ParticleSystem15`) (`self.ParticleSystem16`) (`self.ParticleSystem17`) (`self.ParticleSystem18`) (`self.ParticleSystem19`) (`self.ParticleSystem20`) (`self.ParticleSystem21`) (`self.ParticleSystem22`) (`self.ParticleSystem23`) (`self.ParticleSystem24`) (`self.ParticleSystem25`) (`self.ParticleSystem26`) (`self.ParticleSystem27`) (`self.ParticleSystem28`) (`self.ParticleSystem29`) (`self.ParticleSystem30`) (`self.ParticleSystem31`))))

(event `self.ReceiveBeginPlay`
  (`self.Write Array`)
  (`self.Blinking`))

(event `Blinking`
  (for _array_element (`self.Effects`)
    (`ActorComponent.Deactivate` _array_element)
    (`KismetSystemLibrary.Delay` 1.0)
    (for _array_element_2 (`self.Effects`)
      (`ActorComponent.Activate` _array_element_2 false))
    (`KismetSystemLibrary.Delay` 1.0)
    (`self.Blinking`)))

(fn `UserConstructionScript`)