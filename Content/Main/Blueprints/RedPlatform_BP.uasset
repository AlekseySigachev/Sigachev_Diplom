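; RedPlatform_BP is a moving platform that travels back and forth along a spline, starting on BeginPlay.
; The NormalMovement timeline samples the spline by time in world space to position PlatformMesh each update, without sweeping.
; When the timeline finishes, the MoveForward flag selects reverse or forward playback, creating an endless ping-pong.
; A separate ReverseMovement timeline has the same update logic but is never triggered.
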(event `self.ReceiveBeginPlay`
  (`self.Play`))

(event `Play`
  (set `self.MoveForward` true)
  (bind (_direction _time) (`Timeline|Normal Movement` :!label _label)
    (:`Update`
      (`SceneComponent.K2_SetWorldLocation` (`self.Platform_mesh`) (`SplineComponent.GetLocationAtTime` (`self.Spline`) _time "World" false) false false))
    (:`Finished`
      (if (`self.MoveForward`)
        (`self.Reverse`)
        (else
          (`self.Play`))))))

(event `Reverse`
  (set `self.MoveForward` false)
  (goto _label :!via `Reverse`))

(fn `UserConstructionScript`)