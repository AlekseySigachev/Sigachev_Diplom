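; Sword-wielding AI enemy character with melee, fly-up and homing dash attacks, plus health and death handling.
; FlyUP lifts it on a timeline until high above the ground or landed, then a looping timer steps it toward the player until the Blackboard flags melee range.
; HealthCheck copies damage-adjusted HP to the Blackboard.
; Death enables physics, then asks an AI controller implementing BPI_Spawner for a replacement before destroying enemy and sword.
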(event `self.MeleeAttack`
  (bind (_returnvalue_roll _returnvalue_pitch _returnvalue_yaw) (`KismetMathLibrary.BreakRotator` (`KismetMathLibrary.FindLookAtRotation` (`self.K2_GetActorLocation`) (`self.K2_GetActorLocation` (`GameplayStatics.GetPlayerCharacter` 0)))))
  (`self.K2_SetActorRotation` (`KismetMathLibrary.MakeRotator` 0.0 0.0 _returnvalue_yaw))
  (`|PlayMontage` (`self.Mesh`) "/Game/Main/AI/Enemy/Animations/Attack_PrimaryA_Enemy_Montage.Attack_PrimaryA_Enemy_Montage"))

(event `self.StartDash`
  (`CharacterMovementComponent.SetMovementMode` (`self.CharacterMovement`) "MOVE_Flying" 0)
  (bind _returnvalue (`KismetSystemLibrary.K2_SetTimerDelegate` (delegate `Dashing`) 0.01 true)))

(event `Dashing`
  (if (`BlackboardComponent.GetValueAsBool` (`AIBlueprintHelperLibrary.GetBlackboard` null) "PlayerIsInMeleeRange")
    (`CharacterMovementComponent.SetMovementMode` (`self.CharacterMovement`) "MOVE_Walking" 0)
    (`KismetSystemLibrary.K2_ClearAndInvalidateTimerHandle` (stale `self.StartDash` _returnvalue))
    (else
      (`self.Dash `))))

(event `self.FlyUP`
  (bind _downarrow (`self.DownArrow`))
  (bind _returnvalue (`SceneComponent.K2_GetComponentLocation` _downarrow))
  (`/Engine/EditorBlueprintResources/StandardMacros.DoOnce` false :!label _label
    (:`Completed`
      (`KismetSystemLibrary.Delay` 1.0)
      (`self.Jump`)
      (`Timeline|Flying_TL` :!via `PlayFromStart`
        (:`Update`
          (`KismetSystemLibrary.Delay` 0.05)
          (`self.K2_SetActorLocation` (+ (* (`SceneComponent.GetUpVector` (`self.CapsuleComponent`)) 20.0) (`self.K2_GetActorLocation`)))
          (bind _outhit (`KismetSystemLibrary.LineTraceSingle` _returnvalue (+ (* (`SceneComponent.GetForwardVector` _downarrow) 10000.0) _returnvalue) "TraceTypeQuery2"))
          (if (> (`.Distance` (`GameplayStatics.BreakHitResult` _outhit)) 700.0)
            (`TimelineComponent.Stop` (`self.Flying_TL`) :!label _label_2)
            (`self.ResetFly`)
            (`self.StartDash`)))))))

(event `ResetFly`
  (goto _label :!via `Reset`))

(event `self.OnLanded`
  (params (Hit :type "HitResult Structure (by ref)"))
  (goto _label_2))

(event `self.ReceiveBeginPlay`
  (bind _mesh (`self.Mesh`))
  (bind _returnvalue (`|SpawnActorFromClass` "/Game/Main/Models/Blade_HeroSword10/SK_Blade_HeroSword10_BP.SK_Blade_HeroSword10_BP_C" (`SceneComponent.GetSocketTransform` _mesh "SwordSocket" "RTS_World") "Undefined" "OverrideRootScale" null null))
  (`self.K2_AttachToComponent` _returnvalue _mesh "SwordSocket" "SnapToTarget" "SnapToTarget" "SnapToTarget" true)
  (set `self.CurrentHP` (`self.MaxHP`)))

(event `self.ReceiveAnyDamage`
  (params (Damage :type "Float (single-precision)") (DamageType :type "DamageType Object Reference") (InstigatedBy :type "Controller Object Reference") (DamageCauser :type "Actor Object Reference"))
  (set `self.CurrentHP` (`KismetMathLibrary.FClamp` (- (`self.CurrentHP`) Damage) 0.0 (`self.MaxHP`))))

(event `self.HealthCheck`
  (`BlackboardComponent.SetValueAsFloat` (`AIBlueprintHelperLibrary.GetBlackboard` null) "CurrentHealth" (`self.CurrentHP`)))

(event `self.Death`
  (bind _returnvalue (`AIBlueprintHelperLibrary.GetAIController` self))
  (if (<= (`self.CurrentHP`) 0.0)
    (`PrimitiveComponent.SetSimulatePhysics` (`self.Mesh`) true)
    (`PrimitiveComponent.SetSimulatePhysics` (`self.CapsuleComponent`) true)
    (`KismetSystemLibrary.Delay` 3.0)
    (if (`KismetSystemLibrary.DoesImplementInterface` _returnvalue "/Game/Main/AI/Enemy/BPI_Spawner.BPI_Spawner_C")
      (message `/Game/Main/AI/Enemy/BPI_Spawner.SpawnNewEnemy` _returnvalue)
      (`self.K2_DestroyActor` (stale `self.ReceiveBeginPlay` _returnvalue))
      (`self.K2_DestroyActor` self))))

(fn `Dash `
  (bind _capsulecomponent (`self.CapsuleComponent`))
  (bind _returnvalue (`SceneComponent.K2_GetComponentLocation` _capsulecomponent))
  (bind (_returnvalue_roll _returnvalue_pitch _returnvalue_yaw) (`KismetMathLibrary.BreakRotator` (`KismetMathLibrary.FindLookAtRotation` (`self.K2_GetActorLocation`) (`self.K2_GetActorLocation` (`GameplayStatics.GetPlayerCharacter` 0)))))
  (bind _returnvalue_2 (* (`KismetMathLibrary.Normal` (- (`self.K2_GetActorLocation` (`GameplayStatics.GetPlayerCharacter` 0)) (`self.K2_GetActorLocation`))) 40.0))
  (`KismetSystemLibrary.SphereTraceSingle` _returnvalue (+ _returnvalue _returnvalue_2) (`CapsuleComponent.CapsuleRadius` _capsulecomponent) "TraceTypeQuery2")
  (`self.K2_SetActorRotation` (`KismetMathLibrary.MakeRotator` 0.0 0.0 _returnvalue_yaw))
  (`self.K2_SetActorLocation` (+ _returnvalue_2 _returnvalue)))

(fn `UserConstructionScript`)