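; AI controller for enemies that runs BT_Enemy, seeds its blackboard with melee range and stores the player character as CurrentTarget.
; AI perception updates the "CanSeePlayer?" blackboard key whenever the sensed actor is the main character.
; A fast looping timer sends DeathMessage to the pawn through BPI_CombatInterface.
; SpawnNewEnemy spawns a BP_Enemy at a random navigable point near the current pawn, possesses it and restarts the behavior tree.
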(event `self.ReceiveBeginPlay`
  (`self.RunBehaviorTree` "/Game/Main/AI/Enemy/BT_Enemy.BT_Enemy")
  (set `self.CurrentTarget` (`GameplayStatics.GetPlayerCharacter` 0))
  (`BlackboardComponent.SetValueAsFloat` (`AIBlueprintHelperLibrary.GetBlackboard` null) "MeleeRange" (`self.AI_MeleeRange`))
  (`KismetSystemLibrary.K2_SetTimerDelegate` (delegate `DeathChecker`) 0.01 true))

(event `DeathChecker`
  (bind _returnvalue (`self.K2_GetPawn`))
  (if (`KismetSystemLibrary.DoesImplementInterface` _returnvalue "/Game/Main/AI/Enemy/BPI_CombatInterface.BPI_CombatInterface_C")
    (message `/Game/Main/AI/Enemy/BPI_CombatInterface.Death` _returnvalue)))

(event `self.AIPerception.OnTargetPerceptionUpdated`
  (params (Actor :type "Actor Object Reference") (Stimulus :type "AIStimulus Structure"))
  (cast `/Game/Main/Character/MainCharacter` Actor)
  (`BlackboardComponent.SetValueAsBool` (`AIBlueprintHelperLibrary.GetBlackboard` null) "CanSeePlayer?" (`.bSuccessfullySensed` (break `AIStimulus` Stimulus))))

(event `/Game/Main/AI/Enemy/BPI_Spawner.SpawnNewEnemy`
  (bind _returnvalue (`|SpawnActorFromClass` "/Game/Main/AI/Enemy/BP_Enemy.BP_Enemy_C" (`KismetMathLibrary.Conv_VectorToTransform` (`NavigationSystemV1.K2_GetRandomLocationInNavigableRadius` (`self.K2_GetActorLocation` (`self.K2_GetPawn`)) 1000.0 null null)) "AlwaysSpawn" "OverrideRootScale" self null))
  (`self.Possess` _returnvalue)
  (`self.RunBehaviorTree` "/Game/Main/AI/Enemy/BT_Enemy.BT_Enemy"))

(fn `UserConstructionScript`)